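; BP_Delivery is the delivery station for the Duck Challenge, giving visual feedback when points are scored.
; On BeginPlay it creates a dynamic material instance for the station mesh.
; OnScored adds scaled points to AnimationSpeed and, for positive scores, tints the material white, pink or red by point tier.
; A two-second timer calls ResetMaterial to restore the cyan color with zero alpha.
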(event `self.OnScored`
  (params (Points :type Integer))
  (set `self.AnimationSpeed` (+ (* Points (`self.RotationSpeedMultiplier`)) (`self.AnimationSpeed`)))
  (if (> Points 0)
    (if (< Points 3)
      (set `self.Color` (struct :`R` 1.0 :`G` 1.0 :`B` 1.0 :`A` 1.0))
      (elif (< Points 8)
        (set `self.Color` (struct :`R` 0.969072 :`G` 0.348958 :`B` 1.0 :`A` 1.0))
        (else
          (set `self.Color` (struct :`R` 1.0 :`B` 0.049179 :`A` 1.0)))))
    (`MaterialInstanceDynamic.SetVectorParameterValue` (`self.Material_Dyn`) "Color" (`self.Color`))
    (`KismetSystemLibrary.K2_SetTimer` null "ResetMaterial" 2.0)))

(event `self.ReceiveBeginPlay`
  (bind _returnvalue (`KismetMaterialLibrary.CreateDynamicMaterialInstance` (`PrimitiveComponent.GetMaterial` (`self.DeliveryStationMesh`) 0)))
  (bind _output_get (set `self.Material_Dyn` _returnvalue))
  (`PrimitiveComponent.SetMaterial` (`self.DeliveryStationMesh`) 0 _output_get))

(fn `ResetMaterial`
  (`MaterialInstanceDynamic.SetVectorParameterValue` (`self.Material_Dyn`) "Color" (struct :`R` 0.155926 :`G` 0.887923 :`B` 1.0)))

(fn `UserConstructionScript`)