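; BP_MellowsPawn is a plane pawn with a grappling hook; this Blueprint drives its visual feedback every Tick.
; A lightning beam spans plane and hook while the hook is visible.
; The movement component's Impulse toggles light and warning material parameters near base max charge, and its attaching state switches hook and cable color.
; The hook rotates along the line from pawn to hook; UpdateLaserPointer and the construction script are empty.
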(event `self.ReceiveTick`
  (params (DeltaSeconds :type "Float (single-precision)"))
  (bind _movementcomponent (`self.MovementComponent`))
  (bind _grapplehook (`self.GrappleHook`))
  (bind _custommaterial_dyn (`self.CustomMaterial_Dyn`))
  (bind _lightning (`self.Lightning`))
  (bind _lightning_2 (`self.Lightning`))
  (bind _returnvalue (`ActorComponent.IsActive` _lightning_2))
  (bind _returnvalue_2 (`KismetMathLibrary.SelectFloat` 1.0 0.0 (`MellowsMovementComponent.bIsAttaching` (`self.MovementComponent`))))
  (bind (_returnvalue_roll _returnvalue_pitch _returnvalue_yaw) (`KismetMathLibrary.BreakRotator` (`KismetMathLibrary.FindLookAtRotation` (`self.K2_GetActorLocation`) (`SceneComponent.K2_GetComponentLocation` _grapplehook))))
  (`|ExecutionSequence`
    (:`then_0`
      ;[1 1 1] Update grapple lightning effect
      (`ParticleSystemComponent.SetBeamTargetPoint` _lightning 0 (`SceneComponent.K2_GetComponentLocation` (`self.GrappleHook`)) 0)
      (`ParticleSystemComponent.SetBeamSourcePoint` _lightning 0 (`SceneComponent.K2_GetComponentLocation` (`self.PlaneMesh`)) 0)
      (if (`SceneComponent.IsVisible` (`self.GrappleHook`))
        (if (not _returnvalue)
          (`ActorComponent.Activate` _lightning_2 true))
        (elif _returnvalue
          (`ActorComponent.Deactivate` _lightning_2))))
    (:`then_1`
      ;[1 1 1] Update Impulse status on pawn
      (if (<= (`MellowsMovementComponent.Impulse` _movementcomponent) (* (`MellowsMovementComponent.BaseMaxCharge` _movementcomponent) 0.99))
        (`MaterialInstanceDynamic.SetScalarParameterValue` _custommaterial_dyn "ImpulseLightStrength" 0.0)
        (`MaterialInstanceDynamic.SetScalarParameterValue` _custommaterial_dyn "ImpulseWarningStrength" 0.0)
        (else
          (`MaterialInstanceDynamic.SetScalarParameterValue` _custommaterial_dyn "ImpulseLightStrength" 1.0)
          (`MaterialInstanceDynamic.SetScalarParameterValue` _custommaterial_dyn "ImpulseWarningStrength" 10.0))))
    (:`then_2`
      (`MeshComponent.SetScalarParameterValueOnMaterials` _grapplehook "IsGreen" _returnvalue_2)
      (`SceneComponent.K2_SetWorldRotation` _grapplehook (`KismetMathLibrary.MakeRotator` _returnvalue_roll (+ _returnvalue_pitch -90.0) _returnvalue_yaw) false true)
      (`MeshComponent.SetVectorParameterValueOnMaterials` (`self.Cable`) "Color" (`KismetMathLibrary.MakeVector` (- 1.0 _returnvalue_2) _returnvalue_2)))))

(fn `UpdateLaserPointer`)

(fn `UserConstructionScript`)