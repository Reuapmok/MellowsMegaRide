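; Player controller for Mellows that routes menu input to the HUD.
; The Menu input action opens the menu through BP_MellowsHUD.
; Gamepad D-pad directions and the left face button are hard-bound keys that pass a navigation enum value to the HUD's InGameMenu, when that widget is valid.
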(event `InputAction|Menu`
  (params (Key :type "Key Structure"))
  (:`Pressed`
    (bind _asbp_mellows_hud (cast `/Game/UI/BP_MellowsHUD` (`self.GetHUD`)))
    (`/Game/UI/BP_MellowsHUD.Open Menu` _asbp_mellows_hud)))

(event `Key|Gamepad_DPad_Down`
  (params (Key :type "Key Structure"))
  (:`Pressed`
    (bind _asbp_mellows_hud (cast `/Game/UI/BP_MellowsHUD` (`self.GetHUD`)))
    (bind _ingamemenu (`/Game/UI/BP_MellowsHUD.InGameMenu` _asbp_mellows_hud))
    (`/Engine/EditorBlueprintResources/StandardMacros.IsValid` _ingamemenu
      (:`Is Valid`
        (`/Game/UI/BP_InGameMenu.HandleMenuNavigationInput` _ingamemenu "NewEnumerator1")))))

(event `Key|Gamepad_DPad_Up`
  (params (Key :type "Key Structure"))
  (:`Pressed`
    (bind _asbp_mellows_hud (cast `/Game/UI/BP_MellowsHUD` (`self.GetHUD`)))
    (bind _ingamemenu (`/Game/UI/BP_MellowsHUD.InGameMenu` _asbp_mellows_hud))
    (`/Engine/EditorBlueprintResources/StandardMacros.IsValid` _ingamemenu
      (:`Is Valid`
        (`/Game/UI/BP_InGameMenu.HandleMenuNavigationInput` _ingamemenu "NewEnumerator0")))))

(event `Key|Gamepad_DPad_Right`
  (params (Key :type "Key Structure"))
  (:`Pressed`
    (bind _asbp_mellows_hud (cast `/Game/UI/BP_MellowsHUD` (`self.GetHUD`)))
    (bind _ingamemenu (`/Game/UI/BP_MellowsHUD.InGameMenu` _asbp_mellows_hud))
    (`/Engine/EditorBlueprintResources/StandardMacros.IsValid` _ingamemenu
      (:`Is Valid`
        (`/Game/UI/BP_InGameMenu.HandleMenuNavigationInput` _ingamemenu "NewEnumerator4")))))

(event `Key|Gamepad_DPad_Left`
  (params (Key :type "Key Structure"))
  (:`Pressed`
    (bind _asbp_mellows_hud (cast `/Game/UI/BP_MellowsHUD` (`self.GetHUD`)))
    (bind _ingamemenu (`/Game/UI/BP_MellowsHUD.InGameMenu` _asbp_mellows_hud))
    (`/Engine/EditorBlueprintResources/StandardMacros.IsValid` _ingamemenu
      (:`Is Valid`
        (`/Game/UI/BP_InGameMenu.HandleMenuNavigationInput` _ingamemenu "NewEnumerator3")))))

(event `Key|Gamepad_FaceButton_Left`
  (params (Key :type "Key Structure"))
  (:`Pressed`
    (bind _asbp_mellows_hud (cast `/Game/UI/BP_MellowsHUD` (`self.GetHUD`)))
    (bind _ingamemenu (`/Game/UI/BP_MellowsHUD.InGameMenu` _asbp_mellows_hud))
    (`/Engine/EditorBlueprintResources/StandardMacros.IsValid` _ingamemenu
      (:`Is Valid`
        (`/Game/UI/BP_InGameMenu.HandleMenuNavigationInput` _ingamemenu "NewEnumerator2")))))

(fn `UserConstructionScript`)